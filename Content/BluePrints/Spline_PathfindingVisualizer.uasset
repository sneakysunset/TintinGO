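; Spline actor that, as its name suggests, visualizes a pathfinding route by laying meshes along its spline.
; The construction script adds a spline mesh per section, with section length optionally driven by the actor's X scale.
; Each mesh's forward axis switches between X and Y from the X offset between spline points.
; Helpers place section ends by distance, but clamp tangents sampled only at the spline's start.
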(event EventBeginPlay)

(event Collision|EventActorBeginOverlap
  (params (OtherActor :type Actor%20Object%20Reference)))

(event EventTick
  (params (DeltaSeconds :type Float%20%28single-precision%29)))

(fn ConstructionScript
  (if (Variables|Default|GetAllowScaling)
    (Variables|Default|SetSection%20Length (* (.x (Transformation|GetActorScale3D)) 1e+02)))
  (for _index (range 0 (Math|Float|Truncate (/ (Spline|GetSplineLength (Variables|Default|GetSpline)) (Variables|Default|GetSection%20Length))))
    (LocalVariables|Setindex _index)
    (bind _returnvalue (AddComponent|AddSplineMeshComponent false))
    (Components|StaticMesh|SetStaticMesh _returnvalue (Variables|Default|GetSplineMesh))
    (if (> (Math|Float|Absolute(Float) (.x (- (Spline|GetLocationatSplinePoint (Variables|Default|GetSpline) (LocalVariables|Getindex) "Local") (Spline|GetLocationatSplinePoint (Variables|Default|GetSpline) (+ (LocalVariables|Getindex) 10) "Local")))) 2e+01)
      (Variables|Default|SetIn%20Forward%20Axis "Y")
      (else
        (Variables|Default|SetIn%20Forward%20Axis "X")))
    (SplineMesh|SetForwardAxis _returnvalue (Variables|Default|GetIn%20Forward%20Axis) true)
    (bind (_location _tangeant) (CallFunction|GetStartPosandTangeant (LocalVariables|Getindex)))
    (bind (_position _tangeant_2) (CallFunction|GetEndPosandTangeant (Class|KismetMathLibrary|ToInt64(Integer) (LocalVariables|Getindex))))
    (SplineMesh|SetStartandEnd _returnvalue _location _tangeant _position _tangeant_2 true :!class /Script/Engine.SplineMeshComponent)))

(fn GetStartPosandTangeant
  (params (Index :type Integer))
  (bind _spline (Variables|Default|GetSpline))
  (return (Spline|GetLocationatDistanceAlongSpline _spline (* Index (Variables|Default|GetSection%20Length)) "Local") (Math|Vector|ClampVectorSize (Spline|GetTangentatDistanceAlongSpline _spline 0.0 "Local") 0.0 (Variables|Default|GetSection%20Length))))

(fn GetEndPosandTangeant
  (params (Index :type Integer64))
  (bind _spline (Variables|Default|GetSpline))
  (return (Spline|GetLocationatDistanceAlongSpline _spline (* (+ Index 1) (Variables|Default|GetSection%20Length)) "Local") (Math|Vector|ClampVectorSize (Spline|GetTangentatDistanceAlongSpline _spline 0.0 "Local") 0.0 (Variables|Default|GetSection%20Length))))